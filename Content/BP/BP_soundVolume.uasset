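; BP_soundVolume is an expanding sound-wave actor that passes its origin and radius to the BP_Item actors it reaches.
; Each Tick grows the Sphere collision radius by SoundSpeed per frame, scales Sphere1 to match, and destroys the actor past MaxSize.
; Overlapped items receive the wave position, have Alpha reset to zero, and join OverlapAcs, whose items get the growing radius every frame.
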(event `self.ReceiveActorBeginOverlap`
  (params (OtherActor :type "Actor Object Reference"))
  (bind _asbp_item (cast `/Game/BP/BP_Item` OtherActor))
  (`/Game/BP/BP_Item.setSoundPos` _asbp_item (`self.K2_GetActorLocation`))
  (set `/Game/BP/BP_Item.alpha` 0.0 _asbp_item)
  (`KismetArrayLibrary.Array_Add` (`self.overlapAcs`) _asbp_item))

(event `self.ReceiveTick`
  (params (DeltaSeconds :type "Float (single-precision)"))
  (bind _sphere (`self.Sphere`))
  (bind _sphereradius (`SphereComponent.SphereRadius` _sphere))
  (bind _returnvalue (+ _sphereradius (`self.soundSpeed`)))
  (`SphereComponent.SetSphereRadius` _sphere _returnvalue true)
  (for _array_element (`self.overlapAcs`)
    (bind _asbp_item (cast `/Game/BP/BP_Item` _array_element))
    (`/Game/BP/BP_Item.setSoundRad` _asbp_item _returnvalue))
  (`SceneComponent.SetWorldScale3D` (`self.Sphere1`) (`KismetMathLibrary.Conv_DoubleToVector` (/ _sphereradius 50.0)))
  (if (> _sphereradius (`self.maxSize`))
    (`self.K2_DestroyActor`)))

(fn `UserConstructionScript`)