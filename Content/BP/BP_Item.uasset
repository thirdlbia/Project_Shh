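; BP_Item is an item actor that drives a sound-reveal style material effect on its static mesh through alpha, radius and position parameters.
; Events for alpha, sound radius and sound position write those values to the mesh's materials.
; Tick raises Alpha by a fixed, frame-rate-dependent step until it reaches one, then keeps setting the radius to zero.
; Direct material-instance setters remain as unconnected nodes.
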(event `self.ReceiveBeginPlay`)

(event `self.ReceiveTick`
  (params (DeltaSeconds :type "Float (single-precision)"))
  (bind _alpha (`self.alpha`))
  (if (< _alpha 1.0)
    (bind _output_get (set `self.alpha` (+ _alpha 0.003)))
    (`self.setAlpha` _output_get)
    (else
      (`self.setSoundRad` 0.0))))

(event `self.ReceiveActorBeginOverlap`
  (params (OtherActor :type "Actor Object Reference")))

(event `setAlpha`
  (params (alpha :type "Float (double-precision)" :default 0.0))
  (`MeshComponent.SetScalarParameterValueOnMaterials` (`self.StaticMesh`) "alpha" alpha))

(event `setSoundRad`
  (params (Rad :type "Float (double-precision)"))
  (`MeshComponent.SetScalarParameterValueOnMaterials` (`self.StaticMesh`) "Radius" Rad))

(event `setSoundPos`
  (params (pos :type "Vector Structure"))
  (`MeshComponent.SetVectorParameterValueOnMaterials` (`self.StaticMesh`) "a" pos))

(fn `UserConstructionScript`)